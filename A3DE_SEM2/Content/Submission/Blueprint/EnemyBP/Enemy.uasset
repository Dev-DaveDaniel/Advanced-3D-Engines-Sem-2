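; Enemy Blueprint that the player can kill with a takedown.
; A Box overlap sets CanTakedown on the ThirdPersonCharacter when it enters and clears it when it leaves.
; The Takedown event disables movement and collision, plays the enemy montage, then destroys the actor after a delay.
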(event OnComponentBeginOverlap(Box)
  (params (OverlappedComponent :type Primitive%20Component%20Object%20Reference) (OtherActor :type Actor%20Object%20Reference) (OtherComp :type Primitive%20Component%20Object%20Reference) (OtherBodyIndex :type Integer) (bFromSweep :type Boolean) (SweepResult :type Hit%20Result%20Structure%20%28by%20ref%29))
  (bind _asthird_person_character (Utilities|Casting|CastToThirdPersonCharacter OtherActor))
  (Variables|/Game/ThirdPersonBP/Blueprints/ThirdPersonCharacter.ThirdPersonCharacter_C|SetCanTakedown? _asthird_person_character true))

(event OnComponentEndOverlap(Box)
  (params (OverlappedComponent :type Primitive%20Component%20Object%20Reference) (OtherActor :type Actor%20Object%20Reference) (OtherComp :type Primitive%20Component%20Object%20Reference) (OtherBodyIndex :type Integer))
  (bind _asthird_person_character (Utilities|Casting|CastToThirdPersonCharacter OtherActor))
  (Variables|/Game/ThirdPersonBP/Blueprints/ThirdPersonCharacter.ThirdPersonCharacter_C|SetCanTakedown? _asthird_person_character false))

(event Custom|Takedown
  (Pawn|Components|CharacterMovement|DisableMovement (Variables|Character|GetCharacterMovement))
  (Collision|SetActorEnableCollision false)
  (Animation|PlayAnimMontage "/Game/Submission/Character/Animation/Enemy/Enemy_Strangle/Enemy_Anim_Montage.Enemy_Anim_Montage" 1.0 "None")
  (Utilities|FlowControl|Delay 3e+01)
  (Actor|DestroyActor))

(fn ConstructionScript)